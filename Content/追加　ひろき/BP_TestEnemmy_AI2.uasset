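; BP_TestEnemmy_AI2 is a test enemy that takes point damage and, at zero health, destroys itself, spawns an explosion and increments EnemyCounter on ThirdPersonGameMode.
; Its damage handler prints debug text and subtracts Damage a second time in a follow-up sequence branch, whose low-health check does nothing.
; Tick, AttachWeapon and SetGunAttack do nothing, as the weapon-attach and rifle line-trace firing logic is left disconnected.
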(event `self.ReceivePointDamage`
  (params (Damage :type "Float (single-precision)") (DamageType :type "DamageType Object Reference") (HitLocation :type "Vector Structure") (HitNormal :type "Vector Structure") (HitComponent :type "PrimitiveComponent Object Reference") (BoneName :type Name) (ShotFromDirection :type "Vector Structure") (InstigatedBy :type "Controller Object Reference") (DamageCauser :type "Actor Object Reference") (HitInfo :type "HitResult Structure (by ref)"))
  (bind _returnvalue (- (`self.Health`) Damage))
  (`|ExecutionSequence`
    (:`then_0`
      (bind _output_get (set `self.Health` _returnvalue))
      (`KismetSystemLibrary.PrintString` (`KismetStringLibrary.Conv_DoubleToString` _output_get))
      (if (<= _output_get 0.0)
        (`KismetSystemLibrary.PrintString` "dead")
        (`self.K2_DestroyActor`)
        (`|SpawnActorFromClass` "/Game/StarterContent/Blueprints/Blueprint_Effect_Explosion.Blueprint_Effect_Explosion_C" (`self.GetTransform`) "Undefined" "OverrideRootScale" null null)
        (bind _asthird_person_game_mode (cast `/Game/UndeadPack/Ghoul/Demo/ThirdPersonTemplate/ThirdPersonBP/Blueprints/ThirdPersonGameMode` (`GameplayStatics.GetGameMode`)))
        (`/Engine/EditorBlueprintResources/StandardMacros.IncrementInt` (`/Game/UndeadPack/Ghoul/Demo/ThirdPersonTemplate/ThirdPersonBP/Blueprints/ThirdPersonGameMode.EnemyCounter` _asthird_person_game_mode))))
    (:`then_1`
      (bind _output_get_2 (set `self.Health` _returnvalue))
      (if (<= _output_get_2 60.0)
        _))))

(event `self.ReceiveTick`
  (params (DeltaSeconds :type "Float (single-precision)")))

(fn `AttachWeapon`
  (params (SocketName :type Name) (`HasWeapon?` :type Boolean)))

(fn `SetGunAttack`
  (locals (`Socket Transform Local` :type "Transform Structure")))

(fn `UserConstructionScript`)